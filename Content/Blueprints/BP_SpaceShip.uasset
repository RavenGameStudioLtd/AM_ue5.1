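; BP_SpaceShip is a player-possessable spacecraft with switchable cameras and landing/takeoff.
; Possession adds the Enhanced Input spaceship mapping context, and a flip-flop toggles chase and cockpit cameras, hiding the hull in cockpit view.
; Land/Takeoff toggles IsFlying and plays timelines that offset the actor's transform.
; Thrust is unfinished: Tick smooths and clamps the input, but nothing applies it to movement.
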(event `self.ReceivePossessed`
  (params (NewController :type "Controller Object Reference"))
  (`EnhancedInputSubsystemInterface.AddMappingContext` (pcsubsystem `EnhancedInputLocalPlayerSubsystem` (`GameplayStatics.GetPlayerController` 0)) "/Game/Player/PlayerAssets/Input/IMC_Spaceship.IMC_Spaceship" 2 (struct))
  (`KismetSystemLibrary.PrintString` "Input ACtion Added"))

(event `self.ReceiveBeginPlay`
  (`|ExecutionSequence`
    (:`then_0`
      (set `self.ThrustTarget` (`self.MinimumThrust`)))))

(event `self.ReceiveTick`
  (params (DeltaSeconds :type "Float (single-precision)"))
  (`|ExecutionSequence`
    (:`then_0`
      (bind _output_get (set `self.MoveFowardInterp` (`KismetMathLibrary.FClamp` (`KismetMathLibrary.FInterpTo` (stale _output_get) (`|GetInputActionValue`) (`GameplayStatics.GetWorldDeltaSeconds`))))))))

(event `EnhancedInput|/Game/Player/PlayerAssets/Input/Actions/Spacecraft/IA_Switch_Craft_cam`
  (params (ActionValue :type Boolean) (ElapsedSeconds :type "Float (double-precision)") (TriggeredSeconds :type "Float (double-precision)") (InputAction :type "InputAction Object Reference" :default "/Game/Player/PlayerAssets/Input/Actions/Spacecraft/IA_Switch_Craft_cam.IA_Switch_Craft_cam"))
  (bind _craftview (`self.CraftView`))
  (bind _cockpitview (`self.CockpitView`))
  (bind _spaceship (`self.Spaceship`))
  ;[1 1 1] Switch Camera view between Behind Craft and Cockpit View
  (:`Triggered`
    (`/Engine/EditorBlueprintResources/StandardMacros.FlipFlop`
      (:`A`
        (`ActorComponent.SetActive` _craftview false false)
        (`ActorComponent.SetActive` _cockpitview true false)
        (`SceneComponent.SetVisibility` _spaceship false false))
      (:`B`
        (`ActorComponent.SetActive` _craftview true false)
        (`ActorComponent.SetActive` _cockpitview false false)
        (`SceneComponent.SetVisibility` _spaceship true false)))))

(event `EnhancedInput|/Game/Player/PlayerAssets/Input/Actions/Spacecraft/IA_Thrust_Spacecraft`
  (params (ActionValue :type "Float (double-precision)") (ElapsedSeconds :type "Float (double-precision)") (TriggeredSeconds :type "Float (double-precision)") (InputAction :type "InputAction Object Reference" :default "/Game/Player/PlayerAssets/Input/Actions/Spacecraft/IA_Thrust_Spacecraft.IA_Thrust_Spacecraft"))
  (:`Triggered`
    (if (`self.IsFlying`)
      _)))

(event `EnhancedInput|/Game/Player/PlayerAssets/Input/Actions/Spacecraft/IA_Land_Takeoff_Spacecraft`
  (params (ActionValue :type Boolean) (ElapsedSeconds :type "Float (double-precision)") (TriggeredSeconds :type "Float (double-precision)") (InputAction :type "InputAction Object Reference" :default "/Game/Player/PlayerAssets/Input/Actions/Spacecraft/IA_Land_Takeoff_Spacecraft.IA_Land_Takeoff_Spacecraft"))
  (bind _returnvalue (`self.K2_GetActorLocation`))
  (:`Triggered`
    (if (`self.IsFlying`)
      (set `self.IsFlying` false)
      (bind (_direction _newtrack_0) (`Timeline|Landing` :!via `PlayFromStart`)
        (:`Update`
          (`self.K2_SetActorRelativeTransform` (`KismetMathLibrary.Conv_VectorToTransform` (+ _newtrack_0 _returnvalue)))))
      (else
        (set `self.IsFlying` true)
        (bind (_direction_2 _newtrack_1) (`Timeline|Launching` :!via `PlayFromStart`)
          (:`Update`
            (`self.K2_SetActorRelativeTransform` (`KismetMathLibrary.Conv_VectorToTransform` (+ _newtrack_1 _returnvalue)))))))))

(fn `UserConstructionScript`)